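; BP_Interact is an interactable actor, apparently a base, that detects when the player is within range.
; Its Box overlap events filter for player pawn 0, send it BeginInteractMessage or EndInteractMessage, and show or hide a TextRender prompt.
; The Interact event is the entry point to call for interaction and is left empty here.
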(event OnComponentBeginOverlap(Box)
  (params (OverlappedComponent :type Primitive%20Component%20Object%20Reference) (OtherActor :type Actor%20Object%20Reference) (OtherComp :type Primitive%20Component%20Object%20Reference) (OtherBodyIndex :type Integer) (bFromSweep :type Boolean) (SweepResult :type Hit%20Result%20Structure%20%28by%20ref%29))
  ;[1 1 1] Detecting Player
  (if (== OtherActor (Game|Player|GetPlayerPawn 0))
    (Class|BPIInteract|BeginInteract(Message) OtherActor)
    (Rendering|SetVisibility (Variables|Default|GetTextRender) true false)))

(event OnComponentEndOverlap(Box)
  (params (OverlappedComponent :type Primitive%20Component%20Object%20Reference) (OtherActor :type Actor%20Object%20Reference) (OtherComp :type Primitive%20Component%20Object%20Reference) (OtherBodyIndex :type Integer))
  ;[1 1 1] Detecting Player
  (if (== OtherActor (Game|Player|GetPlayerPawn 0))
    (Class|BPIInteract|EndInteract(Message) OtherActor)
    (Rendering|SetVisibility (Variables|Default|GetTextRender) false false)))

(event EventBeginPlay)

(event Collision|EventActorBeginOverlap
  (params (OtherActor :type Actor%20Object%20Reference)))

(event EventTick
  (params (DeltaSeconds :type Float%20%28single-precision%29)))

(event EventInteract
  ;[1 1 1] THIS IS THE EVENT YOU CALL TO INTERACT WITH THE BLUEPRINT
)

(fn ConstructionScript)