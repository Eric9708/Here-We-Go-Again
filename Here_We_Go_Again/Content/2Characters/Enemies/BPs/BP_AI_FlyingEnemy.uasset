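; Flying enemy AI that shoots projectiles at the player character on sight; this graph holds no movement logic.
; PawnSensing's see-pawn event snaps the actor to face the player, then spawns BP_EnemyProjectile at ProjSpawnLoc if CanAttack is set.
; Damage, zero gravity and speeds are written to the projectile after it spawns.
; The CanAttack flag and a short Delay limit the fire rate.
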(event OnSeePawn(PawnSensing)
  (params (Pawn :type Pawn%20Object%20Reference))
  (bind _asbp_third_person_character (Utilities|Casting|CastToBP_ThirdPersonCharacter Pawn))
  (Transformation|SetActorRotation (Math|Rotator|FindRelativeLookatRotation (Math|Conversions|ToTransform(Vector) (Transformation|GetActorLocation)) (Transformation|GetActorLocation _asbp_third_person_character)))
  (if (Variables|Default|GetCanAttack?)
    (bind _returnvalue (Game|SpawnActorfromClass "/Game/3Blueprints/Projectiles/BP_EnemyProjectile.BP_EnemyProjectile_C" (Transformation|GetWorldTransform (Variables|Default|GetProjSpawnLoc)) "Undefined" "MultiplyWithRoot" 0 0))
    (bind _output_get (Variables|Default|SetProjectileRef _returnvalue))
    (Variables|Default|SetProjectile%20Movement (Variables|/Game/3Blueprints/Projectiles/BP_EnemyProjectile.BP_EnemyProjectile_C|GetProjectileMovement _output_get))
    (Variables|/Game/3Blueprints/Projectiles/BP_EnemyProjectile.BP_EnemyProjectile_C|SetDamage (Variables|Default|GetProjectileRef) 5.0)
    (Variables|/Script/Engine.ProjectileMovementComponent|SetProjectileGravityScale (Variables|Default|GetProjectile%20Movement) 0.0)
    (Variables|/Script/Engine.ProjectileMovementComponent|SetMaxSpeed (Variables|Default|GetProjectile%20Movement) 5e+03)
    (Variables|/Script/Engine.ProjectileMovementComponent|SetInitialSpeed (Variables|Default|GetProjectile%20Movement) 3e+03)
    (Variables|Default|SetCanAttack? false)
    (Utilities|FlowControl|Delay 0.5)
    (Variables|Default|SetCanAttack? true)))

(event EventBeginPlay)

(event Collision|EventActorBeginOverlap
  (params (OtherActor :type Actor%20Object%20Reference)))

(event EventTick
  (params (DeltaSeconds :type Float%20%28single-precision%29)))

(fn ConstructionScript)